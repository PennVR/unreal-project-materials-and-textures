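; LobbyLogic is a lobby actor that shows discovered LAN game sessions as spheres in the world.
; RefreshServerEvent runs FindSessions, stores results on success, and repopulates on either outcome, so a failure redraws the previously stored list.
; RepopulateServers destroys the old spheres, then spawns one Server_Sphere per session, stacked upward from the actor at Distance intervals and holding its session.
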(event `RefreshServerEvent`
  (bind _results (`FindSessionsCallbackProxy.FindSessions` (`GameplayStatics.GetPlayerController` 0) 10 true)
    (:`OnSuccess`
      (bind _output_get (set `self.servers` _results))
      (`KismetSystemLibrary.PrintString` (`KismetStringLibrary.Conv_IntToString` (`KismetArrayLibrary.Array_Length` _output_get))))
    (:`OnFailure`
      (`KismetSystemLibrary.PrintString` "I AM A FAILURE>")))
  (`self.RepopulateServers`))

(fn `RepopulateServers`
  (`self.ClearServerSpheres`
    (:`exec`
      (for (_array_element _array_index) (`self.servers`)
        (`self.SpawnServerSphere` _array_index _array_element)))))

(fn `SpawnServerSphere`
  (params (index :type Integer) (session :type "BlueprintSessionResult Structure"))
  (locals (distance :type "Float (double-precision)" :default 200.0))
  (bind _returnvalue (`self.K2_GetActorLocation`))
  (bind _returnvalue_2 (* (`local.distance`) (`KismetMathLibrary.Conv_IntToDouble` index) 1.0))
  (`KismetSystemLibrary.PrintString` (`KismetStringLibrary.Conv_DoubleToString` _returnvalue_2))
  (`KismetSystemLibrary.PrintString` (`KismetStringLibrary.Conv_VectorToString` _returnvalue))
  (bind _returnvalue_3 (`|SpawnActorFromClass` "/Game/Server_Sphere.Server_Sphere_C" (`KismetMathLibrary.MakeTransform` (+ (`KismetMathLibrary.MakeVector` 0.0 0.0 _returnvalue_2) _returnvalue) (struct) (2.0 2.0 2.0)) "Undefined" "OverrideRootScale" self))
  (set `/Game/Server_Sphere.session` session _returnvalue_3)
  (`KismetArrayLibrary.Array_Add` (`self.ServerSpheres`) _returnvalue_3))

(fn `UserConstructionScript`)