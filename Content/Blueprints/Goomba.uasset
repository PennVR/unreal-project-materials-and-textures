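; Goomba is a pawn that walks toward an AI stop and snaps back to its starting location on arrival.
; BeginPlay stores that location and spawns an AIStop at the world origin as SpawnNode.
; Tick issues AI MoveTo toward SpawnNode's NextStop every frame, teleporting the pawn back on success.
; The step that would advance SpawnNode along the stop chain is unwired, so the target reference never advances.
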(event `self.ReceiveBeginPlay`
  (bind _output_get (set `self.Original location` (`self.K2_GetActorLocation`)))
  (bind _returnvalue (`|SpawnActorFromClass` "/Game/Blueprints/AIStop.AIStop_C" (`KismetMathLibrary.MakeTransform` (0.0 0.0 0.0)) "AlwaysSpawn" "OverrideRootScale"))
  (bind _output_get_2 (set `self.Spawn Node` _returnvalue)))

(event `self.ReceiveTick`
  (params (DeltaSeconds :type "Float (single-precision)"))
  (`|AIMoveTo` self (0.0 0.0 0.0) (`/Game/Blueprints/AIStop.Next Stop` (stale `self.ReceiveBeginPlay` _output_get_2))
    (:`OnSuccess`
      (`self.K2_SetActorLocation` (stale `self.ReceiveBeginPlay` _output_get) false true))))

(fn `UserConstructionScript`)